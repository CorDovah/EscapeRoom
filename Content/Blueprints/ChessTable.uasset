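; ChessTable actor that periodically rotates itself on a countdown of roughly one minute.
; Tick runs through a one-second Delay, so the Seconds counter drops about once per second.
; At zero it adds the Rotator variable's pitch to the actor's current pitch, sets roll and yaw to zero, and restarts the countdown.
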(event `self.ReceiveBeginPlay`)

(event `self.ReceiveTick`
  (params (DeltaSeconds :type "Float (single-precision)"))
  (`KismetSystemLibrary.Delay` 1.0)
  (if (== (`self.Seconds`) 0)
    (`self.K2_SetActorRotation` (`KismetMathLibrary.MakeRotator` 0.0 (+ (.pitch (`self.Rotator`)) (.pitch (`self.K2_GetActorRotation`)))))
    (set `self.Seconds` 60)
    (else
      (set `self.Seconds` (- (`self.Seconds`) 1)))))

(fn `UserConstructionScript`)