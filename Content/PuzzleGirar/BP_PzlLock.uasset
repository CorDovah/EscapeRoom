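; BP_PzlLock is a rotating combination-lock puzzle with three sculpted face pieces that controls a linked chest.
; An interact event pitches the chosen piece left or right by a set step, then checks its relative pitch against that slot's code value within a small tolerance.
; Per-piece results are stored in a boolean array, opening the chest when all are correct and closing it otherwise, with debug prints.
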(event `/Game/PuzzleGirar/InteractablePuzzles.Interact With Puzzle`
  (params (Component :type "PrimitiveComponent Object Reference") (RotateLeft :type Boolean))
  (`self.Rotate` Component RotateLeft))

(fn `CheckCode`
  (params (Component :type "PrimitiveComponent Object Reference"))
  (locals (SelectedMesh :type Integer) (LocalFailed :type Boolean))
  (bind _chest (`self.Chest`))
  (bind (_relativerotation_roll _relativerotation_pitch) (`KismetMathLibrary.BreakRotator` (`SceneComponent.RelativeRotation` Component)))
  (if (== Component (`self.Face_Sculpture_FBX-CORONA__Face`))
    (set `local.SelectedMesh` 0)
    (`KismetArrayLibrary.Array_Set` (`self.IsCorrect`) (`local.SelectedMesh`) (`KismetMathLibrary.NearlyEqual_FloatFloat` (`|GetArrayItem` (`self.Code`) (`local.SelectedMesh`)) _relativerotation_pitch 5.0) :!label _label)
    (for _array_element (`self.IsCorrect`)
      (if (not _array_element)
        (set `local.LocalFailed` true)
        (break)))
    (if (`local.LocalFailed`)
      (`/Game/PuzzleGirar/chest01_cap2_Blueprint.CloseChest` _chest)
      (else
        (`/Game/PuzzleGirar/chest01_cap2_Blueprint.OpenChest` _chest)
        (`KismetSystemLibrary.PrintString` "Correct")))
    (elif (== Component (`self.Face_Sculpture_FBX-CORONA__Face1`))
      (set `local.SelectedMesh` 1)
      (goto _label)
      (elif (== Component (`self.Face_Sculpture_FBX-CORONA__Face3`))
        (set `local.SelectedMesh` 2)
        (goto _label)))))

(fn `Rotate`
  (params (Component :type "PrimitiveComponent Object Reference") (RotateLeft :type Boolean))
  (if RotateLeft
    (`SceneComponent.K2_AddRelativeRotation` Component (`KismetMathLibrary.MakeRotator` 0.0 (* (`self.RotateValue`) -1.0)) false false)
    (else
      (`SceneComponent.K2_AddRelativeRotation` Component (`KismetMathLibrary.MakeRotator` 0.0 (`self.RotateValue`)) false false)))
  (`KismetSystemLibrary.PrintString` (`KismetStringLibrary.Conv_RotatorToString` (`SceneComponent.RelativeRotation` Component)))
  (`self.CheckCode` Component))

(fn `UserConstructionScript`)